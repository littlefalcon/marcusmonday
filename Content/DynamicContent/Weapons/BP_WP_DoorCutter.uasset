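; Door cutter weapon Blueprint that, as it stands, holds only unconnected aiming logic and an empty construction script.
; The unwired graph stores the Weapon component's location as MuzzleLocation, then line traces on Visibility from it toward a point ahead of the player's first-person camera.
; It saves the impact point as HitLocation and draws the trace for debugging, with no cutting or damage logic present.
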(fn `UserConstructionScript`)