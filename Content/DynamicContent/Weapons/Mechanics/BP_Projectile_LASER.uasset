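; BP_Projectile_LASER is the laser weapon's projectile, a child Blueprint that takes its stats from the player's laser.
; On BeginPlay it casts the player character to BP_Player and reads Damage and FireRange through FXCastToLaser.
; It derives StableTime by dividing FireRange by ConvertFireRangeToTime, then runs the parent BeginPlay.
; If the player cast fails, neither the stat setup nor the parent BeginPlay runs.
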(event `self.ReceiveBeginPlay`
  (bind _asbp_player (cast `/Game/DynamicContent/Player/BP_Player` (`GameplayStatics.GetPlayerCharacter` 0)))
  (bind _asbp_weapon (`/Game/DynamicContent/Player/BP_Player.FX_CastToLaser` _asbp_player))
  (set `self.Damage` (`/Game/DynamicContent/Weapons/BP_Weapon.Damage` _asbp_weapon))
  (set `self.StableTime` (/ (`/Game/DynamicContent/Weapons/BP_Weapon.FireRange` _asbp_weapon) (`/Game/DynamicContent/Engine/GlobalMacros.ConvertFireRangeToTime`)))
  (`parent.ReceiveBeginPlay`))

(fn `UserConstructionScript`
  (`parent.UserConstructionScript`))