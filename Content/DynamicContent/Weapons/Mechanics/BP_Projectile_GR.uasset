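; Gauss rifle projectile Blueprint that takes its stats from the player's Gauss rifle.
; On BeginPlay it gets the rifle through BP_Player and runs SetProjectileInfo before calling the parent BeginPlay.
; SetProjectileInfo copies Damage and derives StableTime from FireRange divided by ConvertFireRangeToTime, also sending that value to a debug display.
; FXGetDamageGR is an empty stub.
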(event `self.ReceiveBeginPlay`
  (bind _asbp_player (cast `/Game/DynamicContent/Player/BP_Player` (`GameplayStatics.GetPlayerCharacter` 0)))
  (bind _asbp_weapon (`/Game/DynamicContent/Player/BP_Player.FX_CastToGaussRifle` _asbp_player))
  (`self.SetProjectileInfo` _asbp_weapon)
  (`parent.ReceiveBeginPlay`))

(fn `FX_GetDamageGR`
  (return))

(fn `SetProjectileInfo`
  (params (BP_Weapon :type "/Game/DynamicContent/Weapons/BP_Weapon Object Reference"))
  (bind _returnvalue (/ (`/Game/DynamicContent/Weapons/BP_Weapon.FireRange` BP_Weapon) (`/Game/DynamicContent/Engine/GlobalMacros.ConvertFireRangeToTime`)))
  (set `self.Damage` (`/Game/DynamicContent/Weapons/BP_Weapon.Damage` BP_Weapon))
  (`/Game/DynamicContent/Engine/GlobalMacros.SpeedDebug` (`KismetStringLibrary.Conv_DoubleToString` _returnvalue) true)
  (set `self.StableTime` _returnvalue))

(fn `UserConstructionScript`
  (`parent.UserConstructionScript`))