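; BP_MasterItems is an inventory item actor that shows a pickup prompt in range and heals the player when used.
; Construction packs its custom mesh, image, texts and values into an ItemInfo struct.
; The player's pickup dispatcher adds that struct to the inventory menu, then hides the actor rather than destroying it.
; Items can reload from the struct, take a random GameManager drop, or receive a brief spawn force.
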(event `self.ReceiveBeginPlay`
  (bind _iteminfo (`self.ItemInfo`))
  (bind _pickuptextreference (`self.PickupTextReference`))
  (bind (_itemid _item _itemmesh _itemimage _pickuptext) (break `/Game/DynamicContent/PrototypeContent/Inventory/InventoryStruct` _iteminfo))
  ;[1 1 1] Event Begin Play
  (bind _returnvalue (`|CreateWidget` "/Game/DynamicContent/PrototypeContent/Inventory/PickupText.PickupText_C" (`GameplayStatics.GetPlayerController` 0)))
  (set `self.PickupTextReference` _returnvalue)
  (setmembers `/Game/DynamicContent/PrototypeContent/Inventory/InventoryStruct` :`StructRef` _iteminfo :`Item` self)
  (set `/Game/DynamicContent/PrototypeContent/Inventory/PickupText.PickupActor` _item _pickuptextreference)
  (set `/Game/DynamicContent/PrototypeContent/Inventory/PickupText.PickupText` _pickuptext _pickuptextreference)
  (set `self.ItemID` (`self.ItemID`))
  (bind _asplayer (cast `/Game/DynamicContent/PrototypeContent/Character/Player` (`GameplayStatics.GetPlayerCharacter` 0)))
  (bind _output_get (set `self.CharacterReference` _asplayer))
  (add `/Game/DynamicContent/PrototypeContent/Character/Player.PickupItem` _output_get (delegate `Event_PickupItem`)))

(event `self.Trigger.OnComponentBeginOverlap`
  (params (OverlappedComponent :type "PrimitiveComponent Object Reference") (OtherActor :type "Actor Object Reference") (OtherComp :type "PrimitiveComponent Object Reference") (OtherBodyIndex :type Integer) (bFromSweep :type Boolean) (SweepResult :type "HitResult Structure (by ref)"))
  ;[1 1 1] OverlapTrigger Script
  (cast `/Game/DynamicContent/PrototypeContent/Character/Player` OtherActor)
  (`UserWidget.AddToViewport` (`self.PickupTextReference`) 0)
  (set `self.IsInRange` true))

(event `Event_PickupItem`
  (bind _inventorymenureference (`/Game/DynamicContent/PrototypeContent/Character/Player.InventoryMenuReference` (`self.CharacterReference`)))
  ;[1 1 1] Pickup Item and add to inventory then Refresh inventory
  (if (and (`self.GetActorEnableCollision`) (`self.IsInRange`))
    (`KismetArrayLibrary.Array_Add` (`/Game/DynamicContent/PrototypeContent/UI/InGame/Inventory.Inventory` _inventorymenureference) (`self.ItemInfo`))
    (`Widget.RemoveFromParent` (`self.PickupTextReference`))
    (`self.SetActorHiddenInGame` true)
    (`self.SetActorEnableCollision` false)
    (`/Game/DynamicContent/PrototypeContent/UI/InGame/Inventory.RefreshInventory` _inventorymenureference)))

(event `self.Trigger.OnComponentEndOverlap`
  (params (OverlappedComponent :type "PrimitiveComponent Object Reference") (OtherActor :type "Actor Object Reference") (OtherComp :type "PrimitiveComponent Object Reference") (OtherBodyIndex :type Integer))
  ;[1 1 1] OverlapTrigger Script
  (cast `/Game/DynamicContent/PrototypeContent/Character/Player` OtherActor)
  (`Widget.RemoveFromParent` (`self.PickupTextReference`))
  (set `self.IsInRange` false))

(event `self.ReceiveTick`
  (params (DeltaSeconds :type "Float (single-precision)"))
  (bind _pickuptextreference (`self.PickupTextReference`))
  (bind _returnvalue (`SceneComponent.K2_GetComponentLocation` (`self.ItemMesh`)))
  ;[1 1 1] Random Force Position to Item after Spawn
  (if (`self.IsDrop`)
    (set `/Game/DynamicContent/PrototypeContent/Inventory/PickupText.ItemLocation` _returnvalue _pickuptextreference)
    (`PrimitiveComponent.AddForce` (`self.ItemMesh`) (`self.ForceDirection`) "None" false)
    (`KismetSystemLibrary.Delay` 0.2)
    (set `self.IsDrop` false)
    (else
      (set `/Game/DynamicContent/PrototypeContent/Inventory/PickupText.ItemLocation` _returnvalue _pickuptextreference))))

(event `/Game/DynamicContent/PrototypeContent/Inventory/ActionInterface.UseAction`
  (bind _characterreference (`self.CharacterReference`))
  ;[1 1 1] Use Item
  (set `/Game/DynamicContent/PrototypeContent/Character/Player.HP` (+ (`self.AddHealth`) (`/Game/DynamicContent/PrototypeContent/Character/Player.HP` _characterreference)) _characterreference)
  (`/Game/DynamicContent/PrototypeContent/Character/Player.UpdateHealth` _characterreference true false))

(event `/Game/DynamicContent/PrototypeContent/Inventory/ActionInterface.LoadItemInformation`
  (bind _pickuptextreference (`self.PickupTextReference`))
  (bind (_itemid _item _itemmesh _itemimage _pickuptext _actiontext _addhealth) (break `/Game/DynamicContent/PrototypeContent/Inventory/InventoryStruct` (`self.ItemInfo`)))
  (set `self.ItemID` _itemid)
  (`StaticMeshComponent.SetStaticMesh` (`self.ItemMesh`) _itemmesh)
  (set `self.CustomImage` _itemimage)
  (set `self.AddHealth` _addhealth)
  (bind _output_get (set `self.CustomPickupText` _pickuptext))
  (set `/Game/DynamicContent/PrototypeContent/Inventory/PickupText.PickupText` _output_get _pickuptextreference)
  (set `self.CustomActionText` _actiontext)
  (set `/Game/DynamicContent/PrototypeContent/Inventory/PickupText.PickupActor` _item _pickuptextreference)
  (set `self.CustomImage` _itemimage)
  (set `self.CustomStaticMesh` _itemmesh))

(fn `AddSpawnForce`
  (params (ForceDirection :type "Vector Structure"))
  (set `self.IsDrop` true)
  (set `self.ForceDirection` ForceDirection))

(fn `ExecuteRandomDrop`
  (bind _pickuptextreference (`self.PickupTextReference`))
  (bind _outactors (`GameplayStatics.GetAllActorsOfClass` "/Game/DynamicContent/Engine/GameManager.GameManager_C"))
  (bind (_itemid _customstaticmesh _customimage _custompickuptext _customactiontext _addhealth _addbattery) (`/Game/DynamicContent/Engine/GameManager.GetItemDrop` (`|GetArrayItem` _outactors)))
  (bind _structout (setmembers `/Game/DynamicContent/PrototypeContent/Inventory/InventoryStruct` :`StructRef` (`self.ItemInfo`) :`ItemID` _itemid :`Item` self :`ItemMesh` _customstaticmesh :`ItemImage` _customimage :`PickupText` _custompickuptext :`ActionText` _customactiontext :`AddHealth` _addhealth :`AddBattery` _addbattery))
  (bind (_itemid_2 _item _itemmesh _itemimage _pickuptext _actiontext _addhealth_2 _addbattery_2) (break `/Game/DynamicContent/PrototypeContent/Inventory/InventoryStruct` _structout))
  (`StaticMeshComponent.SetStaticMesh` (`self.ItemMesh`) _itemmesh)
  (set `/Game/DynamicContent/PrototypeContent/Inventory/PickupText.PickupActor` _item _pickuptextreference)
  (set `/Game/DynamicContent/PrototypeContent/Inventory/PickupText.PickupText` _pickuptext _pickuptextreference)
  (set `self.ItemID` _itemid_2)
  (set `self.AddBattery` _addbattery_2)
  (set `self.AddHealth` _addhealth_2)
  (set `self.CustomImage` _itemimage))

(fn `UserConstructionScript`
  (bind _structout (setmembers `/Game/DynamicContent/PrototypeContent/Inventory/InventoryStruct` :`StructRef` (`self.ItemInfo`) :`ItemID` (`self.ItemID`) :`Item` self :`ItemMesh` (`self.CustomStaticMesh`) :`ItemImage` (`self.CustomImage`) :`PickupText` (`self.CustomPickupText`) :`ActionText` (`self.CustomActionText`) :`AddHealth` (`self.AddHealth`)))
  (`StaticMeshComponent.SetStaticMesh` (`self.ItemMesh`) (`.ItemMesh_25_E449C8824AA54D96F9DAAD9604AEFA6D` (break `/Game/DynamicContent/PrototypeContent/Inventory/InventoryStruct` _structout))))