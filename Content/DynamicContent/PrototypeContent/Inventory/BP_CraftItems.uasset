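; Crafting material pickup that adds its amount to the player's CraftInventory.
; Construction asks the GameManager for the drop's type and amount, then builds its label text.
; Trigger overlap shows a pickup widget tracking the mesh, and the player's bound pickup event collects the item in range, then hides it and disables collision.
; AddSpawnForce makes Tick briefly push the mesh in a supplied direction.
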(event `self.ReceiveBeginPlay`
  (bind _pickuptextreference (`self.PickupTextReference`))
  ;[1 1 1] Event Begin Play
  (bind _returnvalue (`|CreateWidget` "/Game/DynamicContent/PrototypeContent/Inventory/PickupText.PickupText_C" (`GameplayStatics.GetPlayerController` 0)))
  (set `self.PickupTextReference` _returnvalue)
  (set `/Game/DynamicContent/PrototypeContent/Inventory/PickupText.PickupActor` self _pickuptextreference)
  (set `/Game/DynamicContent/PrototypeContent/Inventory/PickupText.PickupText` (`KismetTextLibrary.Conv_StringToText` (`KismetStringLibrary.Concat_StrStr` (`self.ItemText`) " " (`self.AmountText`) " EA")) _pickuptextreference)
  (bind _asplayer (cast `/Game/DynamicContent/PrototypeContent/Character/Player` (`GameplayStatics.GetPlayerCharacter` 0)))
  (bind _output_get (set `self.CharacterReference` _asplayer))
  (add `/Game/DynamicContent/PrototypeContent/Character/Player.PickupItem` _output_get (delegate `Event_PickupItem`)))

(event `self.Trigger.OnComponentBeginOverlap`
  (params (OverlappedComponent :type "PrimitiveComponent Object Reference") (OtherActor :type "Actor Object Reference") (OtherComp :type "PrimitiveComponent Object Reference") (OtherBodyIndex :type Integer) (bFromSweep :type Boolean) (SweepResult :type "HitResult Structure (by ref)"))
  ;[1 1 1] OverlapTrigger Script
  (cast `/Game/DynamicContent/PrototypeContent/Character/Player` OtherActor)
  (`UserWidget.AddToViewport` (`self.PickupTextReference`) 0)
  (set `self.IsInRange` true))

(event `Event_PickupItem`
  (bind _craftitem (`self.CraftItem`))
  (bind _craftinventory (`/Game/DynamicContent/PrototypeContent/Character/Player.CraftInventory` (`self.CharacterReference`)))
  ;[1 1 1] Pickup Item and add to inventory then Refresh inventory
  (if (and (`self.GetActorEnableCollision`) (`self.IsInRange`))
    (`KismetArrayLibrary.Array_Set` _craftinventory _craftitem (+ (`|GetArrayItem` _craftinventory _craftitem) (`self.Amount`)))
    (`Widget.RemoveFromParent` (`self.PickupTextReference`))
    (`self.SetActorHiddenInGame` true)
    (`self.SetActorEnableCollision` false)))

(event `self.Trigger.OnComponentEndOverlap`
  (params (OverlappedComponent :type "PrimitiveComponent Object Reference") (OtherActor :type "Actor Object Reference") (OtherComp :type "PrimitiveComponent Object Reference") (OtherBodyIndex :type Integer))
  ;[1 1 1] OverlapTrigger Script
  (cast `/Game/DynamicContent/PrototypeContent/Character/Player` OtherActor)
  (`Widget.RemoveFromParent` (`self.PickupTextReference`))
  (set `self.IsInRange` false))

(event `self.ReceiveTick`
  (params (DeltaSeconds :type "Float (single-precision)"))
  (bind _pickuptextreference (`self.PickupTextReference`))
  (bind _returnvalue (`SceneComponent.K2_GetComponentLocation` (`self.ItemMesh`)))
  ;[1 1 1] Random Force Position to Item after Spawn
  (if (`self.IsDrop`)
    (set `/Game/DynamicContent/PrototypeContent/Inventory/PickupText.ItemLocation` _returnvalue _pickuptextreference)
    (`PrimitiveComponent.AddForce` (`self.ItemMesh`) (`self.ForceDirection`) "None" false)
    (`KismetSystemLibrary.Delay` 0.2)
    (set `self.IsDrop` false)
    (else
      (set `/Game/DynamicContent/PrototypeContent/Inventory/PickupText.ItemLocation` _returnvalue _pickuptextreference))))

(event `/Game/DynamicContent/PrototypeContent/Inventory/ActionInterface.LoadItemInformation`)

(fn `AddSpawnForce`
  (params (ForceDirection :type "Vector Structure"))
  (set `self.IsDrop` true)
  (set `self.ForceDirection` ForceDirection))

(fn `GetItemText`
  (params (ItemIndex :type Integer))
  (returns (ItemText :type String))
  (if (== ItemIndex 0)
    (return "Scrap")
    (elif (== ItemIndex 1)
      (return "Battery")
      (elif (== ItemIndex 2)
        (return "Torch")
        (elif (== ItemIndex 3)
          (return "Wire")
          (elif (== ItemIndex 4)
            (return "Circuit")
            (elif (== ItemIndex 5)
              (return "Laser")
              (elif (== ItemIndex 6)
                (return "Magnet")
                (elif (== ItemIndex 7)
                  (return "Wave")
                  (else
                    (`KismetSystemLibrary.PrintString` "No Index from input")))))))))))

(fn `UserConstructionScript`
  (bind _outactors (`GameplayStatics.GetAllActorsOfClass` "/Game/DynamicContent/Engine/GameManager.GameManager_C"))
  (bind (_craftindex _dropamount) (`/Game/DynamicContent/Engine/GameManager.GetCraftDrop` (`|GetArrayItem` _outactors)))
  (bind _output_get (set `self.CraftItem` _craftindex))
  (bind _output_get_2 (set `self.Amount` _dropamount))
  (bind _itemtext (`self.GetItemText` _output_get))
  (bind _output_get_3 (set `self.ItemText` _itemtext))
  (bind _output_get_4 (set `self.AmountText` (`KismetStringLibrary.Conv_IntToString` _output_get_2)))
  (`StaticMeshComponent.SetStaticMesh` (`self.ItemMesh`) (`self.CustomStaticMesh`))
  (`KismetSystemLibrary.PrintString` (`KismetStringLibrary.Concat_StrStr` _output_get_3 " " _output_get_4 " EA") true false))