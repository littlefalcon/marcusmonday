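; Prototype target dummy that takes projectile damage and drops loot when killed.
; Hits on its mesh from FS__Projectile subtract fixed health, with an explosion effect at the impact point.
; On death it destroys the mesh, adds smoke, and spawns a BP_CraftItems and a randomized BP_MasterItems, launched with random upward-biased forces.
; The actor destroys itself after a short delay.
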(event `self.DummyMesh.OnComponentHit`
  (params (HitComponent :type "PrimitiveComponent Object Reference") (OtherActor :type "Actor Object Reference") (OtherComp :type "PrimitiveComponent Object Reference") (NormalImpulse :type "Vector Structure") (Hit :type "HitResult Structure (by ref)"))
  (bind (_bblockinghit _binitialoverlap _time _distance _location _impactpoint) (`GameplayStatics.BreakHitResult` Hit))
  (bind _returnvalue (- (`self.Health`) 10.0))
  (bind _returnvalue_2 (`KismetMathLibrary.MakeTransform` _impactpoint))
  ;[1 1 1] Hit Mechanic
  (cast `/Game/DynamicContent/PrototypeContent/Weapon/FS__Projectile` OtherActor)
  (bind _output_get (set `self.Health` _returnvalue))
  (if (<= _returnvalue 0.0)
    (`ActorComponent.K2_DestroyComponent` (`self.DummyMesh`))
    (`KismetSystemLibrary.PrintString` (`KismetStringLibrary.Concat_StrStr` "Dead and Drop  " "HP = " (`KismetStringLibrary.Conv_DoubleToString` _output_get)))
    (`GameplayStatics.SpawnEmitterAtLocation` "/Game/StaticContent/StarterContent/Particles/P_Explosion.P_Explosion" _impactpoint)
    (bind _returnvalue_3 (`GameplayStatics.SpawnEmitterAtLocation` "/Game/StaticContent/StarterContent/Particles/P_Smoke.P_Smoke" _impactpoint))
    (bind _returnvalue_4 (`|SpawnActorFromClass` "/Game/DynamicContent/PrototypeContent/Inventory/BP_CraftItems.BP_CraftItems_C" _returnvalue_2 "Undefined" "OverrideRootScale" null 0 null))
    (`/Game/DynamicContent/PrototypeContent/Inventory/BP_CraftItems.AddSpawnForce` _returnvalue_4 (`KismetMathLibrary.MakeVector` (`KismetMathLibrary.Conv_IntToDouble` (`KismetMathLibrary.RandomInteger` 8000)) (`KismetMathLibrary.Conv_IntToDouble` (`KismetMathLibrary.RandomInteger` 8000)) (`KismetMathLibrary.Conv_IntToDouble` (+ (`KismetMathLibrary.RandomInteger` 13000) 10000))))
    (bind _returnvalue_5 (`|SpawnActorFromClass` "/Game/DynamicContent/PrototypeContent/Inventory/BP_MasterItems.BP_MasterItems_C" _returnvalue_2 "Undefined" "OverrideRootScale" null null))
    (`/Game/DynamicContent/PrototypeContent/Inventory/BP_MasterItems.ExecuteRandomDrop` _returnvalue_5)
    (`/Game/DynamicContent/PrototypeContent/Inventory/BP_MasterItems.AddSpawnForce` _returnvalue_5 (`KismetMathLibrary.MakeVector` (`KismetMathLibrary.Conv_IntToDouble` (`KismetMathLibrary.RandomInteger` 8000)) (`KismetMathLibrary.Conv_IntToDouble` (`KismetMathLibrary.RandomInteger` 8000)) (`KismetMathLibrary.Conv_IntToDouble` (+ (`KismetMathLibrary.RandomInteger` 13000) 10000))))
    (`KismetSystemLibrary.Delay` 2.0)
    (`self.K2_DestroyActor`)
    (`ActorComponent.K2_DestroyComponent` _returnvalue_3)
    (else
      (`GameplayStatics.SpawnEmitterAtLocation` "/Game/StaticContent/StarterContent/Particles/P_Explosion.P_Explosion" _impactpoint))))

(fn `UserConstructionScript`)