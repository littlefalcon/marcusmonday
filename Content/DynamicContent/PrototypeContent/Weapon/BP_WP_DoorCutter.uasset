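; Prototype door cutter weapon Blueprint with aiming logic that no event triggers, so it currently does nothing at runtime.
; The unconnected graph stores the weapon component's location as the muzzle point and gets the player's first-person camera.
; It line-traces on Visibility from the weapon toward a point ahead of that camera, with debug drawing, and stores the impact point as the hit location.
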(fn `UserConstructionScript`)