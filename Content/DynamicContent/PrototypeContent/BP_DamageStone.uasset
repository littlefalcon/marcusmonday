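; BP_DamageStone is a prototype damageable stone that displays its remaining HP on a text element.
; Each hit on its static mesh subtracts a fixed placeholder damage amount, updates the text, prints a debug message and destroys the hitting actor.
; Once HP falls to a hard-coded threshold, it destroys the mesh component rather than the whole actor.
; A TODO notes that damage should come from the weapon.
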(event `self.ReceiveBeginPlay`
  (`TextRenderComponent.K2_SetText` (`self.Text_EnemyHP`) (`KismetTextLibrary.Conv_IntToText` (`self.HP`))))

(event `self.StaticMeshComponent.OnComponentHit`
  (params (HitComponent :type "PrimitiveComponent Object Reference") (OtherActor :type "Actor Object Reference") (OtherComp :type "PrimitiveComponent Object Reference") (NormalImpulse :type "Vector Structure") (Hit :type "HitResult Structure (by ref)"))
  (bind _returnvalue (- (`self.HP`) 5))
  (`TextRenderComponent.K2_SetText` (`self.Text_EnemyHP`) (`KismetTextLibrary.Conv_IntToText` _returnvalue))
  (set `self.HP` _returnvalue)
  (`KismetSystemLibrary.PrintString` "Hit")
  (`self.K2_DestroyActor` OtherActor)
  (if (not (> (`self.HP`) 9500))
    (`ActorComponent.K2_DestroyComponent` HitComponent)))

(fn `UserConstructionScript`)