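; BP_CraftVent is a world actor that marks a zone where the player can open the workbench for crafting.
; Its Box overlap events set CanOpenWorkbench on BP_Player to true on entry and false on exit.
; On BeginPlay it caches the UMG_WorldText from its WorldText widget component and fills it with ShowText.
; Leaving the box also prints a debug message and reapplies that same text.
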(event `self.ReceiveBeginPlay`
  (bind _asumg_world_text (cast `/Game/DynamicContent/UI/UMG_WorldText` (`WidgetComponent.GetUserWidgetObject` (`self.WorldText`))))
  (bind _output_get (set `self.TextWidget` _asumg_world_text))
  (`/Game/DynamicContent/UI/UMG_WorldText.SetTextWidget` _output_get (`self.ShowText`)))

(event `self.Box.OnComponentBeginOverlap`
  (params (OverlappedComponent :type "PrimitiveComponent Object Reference") (OtherActor :type "Actor Object Reference") (OtherComp :type "PrimitiveComponent Object Reference") (OtherBodyIndex :type Integer) (bFromSweep :type Boolean) (SweepResult :type "HitResult Structure (by ref)"))
  (bind _asbp_player (cast `/Game/DynamicContent/Player/BP_Player` OtherActor))
  (set `/Game/DynamicContent/Player/BP_Player.CanOpenWorkbench` true _asbp_player))

(event `self.Box.OnComponentEndOverlap`
  (params (OverlappedComponent :type "PrimitiveComponent Object Reference") (OtherActor :type "Actor Object Reference") (OtherComp :type "PrimitiveComponent Object Reference") (OtherBodyIndex :type Integer))
  (bind _asbp_player (cast `/Game/DynamicContent/Player/BP_Player` OtherActor))
  (set `/Game/DynamicContent/Player/BP_Player.CanOpenWorkbench` false _asbp_player)
  (`/Game/DynamicContent/Engine/GlobalMacros.FastDebug` "can open")
  (`/Game/DynamicContent/UI/UMG_WorldText.SetTextWidget` (`self.TextWidget`) (`self.ShowText`)))

(fn `UserConstructionScript`)