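; Infected enemy character driven by an InfectedController and blackboard, which receives heard-noise locations and projectile-hit flags.
; Projectile overlaps on the mesh reduce health, play a hit reaction and spawn particles.
; Death spawns smoke, a random usable item and crafting drops rolled by GameManager, then destroys the actor and reports the kill.
; Attacks play a sword swing, during which socket-attached weapon collision damages the player once.
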(event `self.Mesh.OnComponentBeginOverlap`
  (params (OverlappedComponent :type "PrimitiveComponent Object Reference") (OtherActor :type "Actor Object Reference") (OtherComp :type "PrimitiveComponent Object Reference") (OtherBodyIndex :type Integer) (bFromSweep :type Boolean) (SweepResult :type "HitResult Structure (by ref)"))
  (bind _returnvalue (`self.GetWorldLocation`))
  ;[1 1 1] Hit Mechanic
  (bind (_returnvalue_2 _asbp_projectile) (`self.HitbyProjectile` OtherActor))
  (`self.AIHitReaction`)
  (`self.PlayAnimMontage` (`self.ReactMontage`) 1.0 (`self.AnimSectionName`))
  (if _returnvalue_2
    (`ActorComponent.K2_DestroyComponent` (`self.Mesh`))
    (`PrimitiveComponent.SetCollisionEnabled` (`self.CapsuleComponent`) "NoCollision")
    (bind _hitparticle (`/Game/DynamicContent/Weapons/Mechanics/BP_Projectile.HitParticle` _asbp_projectile))
    (`GameplayStatics.SpawnEmitterAtLocation` _hitparticle _returnvalue)
    (bind _returnvalue_3 (`GameplayStatics.SpawnEmitterAtLocation` "/Game/StaticContent/StarterContent/Particles/P_Smoke.P_Smoke" _returnvalue))
    (`/Game/DynamicContent/Engine/GlobalMacros.DestroyProjectile` _asbp_projectile _asbp_projectile)
    (`self.SpawnCraftItem` (`self.LocToTransfrom` _returnvalue) (`KismetMathLibrary.MakeVector` (`KismetMathLibrary.Conv_IntToDouble` (`KismetMathLibrary.RandomInteger` 500)) (`KismetMathLibrary.Conv_IntToDouble` (`KismetMathLibrary.RandomInteger` 500)) (`KismetMathLibrary.Conv_IntToDouble` (+ (`KismetMathLibrary.RandomInteger` 1000) 1000))))
    (bind _returnvalue_4 (`|SpawnActorFromClass` "/Game/DynamicContent/Engine/Inventory/BP_UsableItem.BP_UsableItem_C" (`KismetMathLibrary.MakeTransform` _returnvalue (struct) (0.15 0.15 0.15)) "Undefined" "OverrideRootScale" null null))
    (`/Game/DynamicContent/Engine/Inventory/BP_UsableItem.ExecuteRandomDrop` _returnvalue_4)
    (`/Game/DynamicContent/Engine/Inventory/BP_UsableItem.AddSpawnForce` _returnvalue_4 (`KismetMathLibrary.MakeVector` (`KismetMathLibrary.Conv_IntToDouble` (`KismetMathLibrary.RandomInteger` 500)) (`KismetMathLibrary.Conv_IntToDouble` (`KismetMathLibrary.RandomInteger` 500)) (`KismetMathLibrary.Conv_IntToDouble` (+ (`KismetMathLibrary.RandomInteger` 1000) 1000))))
    (`KismetSystemLibrary.Delay` 2.0)
    (`self.K2_DestroyActor`)
    (`ActorComponent.K2_DestroyComponent` _returnvalue_3)
    (bind _outactors (`GameplayStatics.GetAllActorsOfClass` "/Game/DynamicContent/Engine/GameManager.GameManager_C"))
    (`/Game/DynamicContent/Engine/GameManager.KilledInfected` (`|GetArrayItem` _outactors))
    (else
      (`GameplayStatics.SpawnEmitterAtLocation` _hitparticle _returnvalue)
      (`/Game/DynamicContent/Engine/GlobalMacros.DestroyProjectile` _asbp_projectile _asbp_projectile))))

(event `Walk`
  (set `CharacterMovementComponent.MaxWalkSpeed` 200.0 (`self.CharacterMovement`)))

(event `Run`
  (set `CharacterMovementComponent.MaxWalkSpeed` 500.0 (`self.CharacterMovement`)))

(event `Attack`
  (bind _mesh (`self.Mesh`))
  (bind _mesh_2 (`self.Mesh`))
  (`/Engine/EditorBlueprintResources/StandardMacros.IsValid` _mesh
    (:`Is Valid`
      (`self.PlayAttackAnimation` _mesh "/Game/StaticContent/MixamoAnimPack/Mixamo_Alpha/Anims/mixamo_Sword_Swing.mixamo_Sword_Swing")
      (set `self.Attacking` true)
      (`KismetSystemLibrary.Delay` 1.5)
      (`/Engine/EditorBlueprintResources/StandardMacros.IsValid` _mesh_2
        (:`Is Valid`
          (`SkeletalMeshComponent.SetAnimationMode` _mesh_2 "AnimationBlueprint"))))))

(event `On Spawned`
  (`/Game/DynamicContent/AI/InfectedController.On Spawned` (stale `self.ReceiveBeginPlay` _output_get)))

(event `self.ReceiveBeginPlay`
  (bind _asinfected_controller (cast `/Game/DynamicContent/AI/InfectedController` (`AIBlueprintHelperLibrary.GetAIController` self)))
  (bind _output_get (set `self.InfectedController` _asinfected_controller)))

(event `self.WeaponCollision.OnComponentBeginOverlap`
  (params (OverlappedComponent :type "PrimitiveComponent Object Reference") (OtherActor :type "Actor Object Reference") (OtherComp :type "PrimitiveComponent Object Reference") (OtherBodyIndex :type Integer) (bFromSweep :type Boolean) (SweepResult :type "HitResult Structure (by ref)"))
  (if (`self.Attacking`)
    (bind _asbp_player (cast `/Game/DynamicContent/Player/BP_Player` OtherActor))
    (`/Game/DynamicContent/Player/BP_Player.TakeDamage` _asbp_player)
    (set `self.Attacking` false)))

(event `self.PawnSensing.OnSeePawn`
  (params (Pawn :type "Pawn Object Reference")))

(event `self.PawnSensing.OnHearNoise`
  (params (Instigator :type "Pawn Object Reference") (Location :type "Vector Structure (by ref)") (Volume :type "Float (single-precision)"))
  (bind _returnvalue (`AIBlueprintHelperLibrary.GetBlackboard` null))
  (set `self.SoundMaker` Instigator)
  (bind _output_get (set `self.SoundLocation` Location))
  (`BlackboardComponent.SetValueAsVector` _returnvalue "SoundLocation" _output_get)
  (`BlackboardComponent.SetValueAsBool` _returnvalue "IsHear" true))

(fn `GetSpawnArea`
  (returns (SpawnArea :type Name))
  (return (`self.SpawnAreaTag`)))

(fn `PlayAttackAnimation`
  (params (InfectedActor :type "SkeletalMeshComponent Object Reference") (NewAnimToPlay :type "AnimationAsset Object Reference"))
  (`SkeletalMeshComponent.PlayAnimation` InfectedActor NewAnimToPlay false)
  (`/Game/DynamicContent/Engine/GlobalMacros.FastDebug` "aaaaaa"))

(fn `UserConstructionScript`
  (`SceneComponent.K2_AttachToComponent` (`self.Weapon`) (`self.Mesh`) (`self.HitSocket`) "KeepRelative" "KeepRelative" "KeepRelative" true))