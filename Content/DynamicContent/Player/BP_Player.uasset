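; Player Blueprint for a space horror game, handling movement sound, health, inventory items, menus and save restoration.
; While accelerating, Tick emits pawn noise and plays surface-based footsteps picked by a line trace, which runs upward from the pawn.
; Key presses open cached widgets for pause, inventory, crafting, upgrades, map and debug.
; Save loading restores stats and child-actor weapon ammo and variants, rebuilding inventory by spawning item actors from hard-coded ID lookups.
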(event `GenerateNoise`
  (params (Instigator :type "Actor Object Reference") (Volume :type "Float (double-precision)") (Location :type "Vector Structure"))
  (`PawnNoiseEmitterComponent.MakeNoise` (`self.PawnNoiseEmitter`) Instigator Volume Location))

(event `self.ReceiveTick`
  (params (DeltaSeconds :type "Float (single-precision)"))
  (bind _walksoundreference (`self.WalkSoundReference`))
  (`self.Event Footstep`)
  (if (or (!= (.x (`CharacterMovementComponent.GetCurrentAcceleration` (`self.CharacterMovement`))) 0.0) (!= (.y (`CharacterMovementComponent.GetCurrentAcceleration` (`self.CharacterMovement`))) 0.0))
    (`self.GenerateNoise` self self 1.0 (`self.K2_GetActorLocation`))
    (else
      (`/Engine/EditorBlueprintResources/StandardMacros.IsValid` _walksoundreference
        (:`Is Valid`
          (`AudioComponent.Stop` _walksoundreference)
          (set `self.IsStop` true))))))

(event `Event Footstep`
  (bind _returnvalue (`GameplayStatics.GetPlayerPawn` 0))
  (bind _returnvalue_2 (`self.K2_GetActorLocation` _returnvalue))
  (if (and (or (!= (.x (`CharacterMovementComponent.GetCurrentAcceleration` (`self.CharacterMovement`))) 0.0) (!= (.y (`CharacterMovementComponent.GetCurrentAcceleration` (`self.CharacterMovement`))) 0.0)) (`self.IsStop`))
    (set `self.IsStop` false)
    (bind _outhit (`KismetSystemLibrary.LineTraceSingle` _returnvalue_2 (+ _returnvalue_2 (0.0 0.0 500.0)) "TraceTypeQuery1" false (`|MakeArray` _returnvalue :!type "Actor Object Reference")))
    (bind _returnvalue_3 (select `EPhysicalSurface` (`GameplayStatics.GetSurfaceType` _outhit) :`SurfaceType_Default` "/Game/DynamicContent/Player/FootStep_Room.FootStep_Room" :`SurfaceType1` "/Game/DynamicContent/Player/FootStep_Room.FootStep_Room" :`SurfaceType2` "/Game/DynamicContent/Player/FootStep_Wood.FootStep_Wood" :!type "SoundBase Object Reference"))
    (bind _returnvalue_4 (`GameplayStatics.SpawnSoundAtLocation` _returnvalue_3 (`.ImpactPoint` (`GameplayStatics.BreakHitResult` _outhit)) (struct) 1.0 1.0 0.0 null null false))
    (set `self.WalkSoundReference` _returnvalue_4)
    (`KismetSystemLibrary.Delay` (`SoundBase.Duration` _returnvalue_3))
    (set `self.IsStop` true)))

(event `Key|G`
  (params (Key :type "Key Structure"))
  ;[1 1 1] TEST take damage
  (:`Pressed`
    (`self.TakeDamage`)))

(event `Key|Q`
  (params (Key :type "Key Structure"))
  (bind _returnvalue (`GameplayStatics.GetPlayerController` 0))
  ;[1 1 1] InGame Menu
  (:`Pressed`
    (`/Engine/EditorBlueprintResources/StandardMacros.IsValid` (`self.PauseMenuReference`)
      (:`Is Valid`
        _)
      (:`Is Not Valid`
        (bind _returnvalue_2 (`|CreateWidget` "/Game/DynamicContent/UI/InGame/InGameMenu.InGameMenu_C"))
        (bind _output_get (set `self.PauseMenuReference` _returnvalue_2))))
    (`WidgetBlueprintLibrary.SetInputMode_UIOnlyEx` _returnvalue _output_get)
    (`UserWidget.AddToViewport` _output_get 0)
    (set `PlayerController.bShowMouseCursor` true _returnvalue)))

(event `Key|Tab`
  (params (Key :type "Key Structure"))
  (bind _inventorymenureference (`self.InventoryMenuReference`))
  (bind _inventorymenureference_2 (`self.InventoryMenuReference`))
  ;[1 1 1] Inventory Menu
  (:`Pressed`
    (`/Engine/EditorBlueprintResources/StandardMacros.IsValid` (`self.InventoryMenuReference`)
      (:`Is Valid`
        _)
      (:`Is Not Valid`
        (bind _returnvalue (`|CreateWidget` "/Game/DynamicContent/UI/InGame/Inventory.Inventory_C"))
        (bind _output_get (set `self.InventoryMenuReference` _returnvalue))))
    (if (and (`/Game/DynamicContent/UI/InGame/Inventory.ActivateInventory` _output_get) (!= (`self.bInventoryDelay`) true))
      (`/Engine/EditorBlueprintResources/StandardMacros.FlipFlop`
        (:`A`
          (set `/Game/DynamicContent/UI/InGame/Inventory.InventoryVisible` "Visible" _output_get)
          (`self.EnebleMouseCursor`)
          (`UserWidget.AddToViewport` _output_get 0)
          (`UserWidget.PlayAnimation` _inventorymenureference_2 (`/Game/DynamicContent/UI/InGame/Inventory.SlideupHologram` _inventorymenureference_2) 0.0 1 "Forward" 1.0)
          (set `self.bInventoryDelay` true)
          (set `self.bMenuOpen` true))
        (:`B`
          (set `self.bInventoryDelay` true)
          (`UserWidget.PlayAnimation` _inventorymenureference (`/Game/DynamicContent/UI/InGame/Inventory.SlideupHologram` _inventorymenureference) 0.0 1 "Reverse" 1.0)
          (`KismetSystemLibrary.Delay` 1.0)
          (set `/Game/DynamicContent/UI/InGame/Inventory.InventoryVisible` "Hidden" _inventorymenureference_2)
          (`self.DisableMouseCursor`)
          (`Widget.RemoveFromParent` _inventorymenureference_2)
          (set `self.bMenuOpen` false)))
      (`KismetSystemLibrary.Delay` 1.0)
      (set `self.bInventoryDelay` false))))

(event `Key|E`
  (params (Key :type "Key Structure"))
  ;[1 1 1] Inventory Menu
  ;;[1 1 1] PickupItem
  (:`Pressed`
    (if (< (`KismetArrayLibrary.Array_Length` (`/Game/DynamicContent/UI/InGame/Inventory.Inventory` (`self.InventoryMenuReference`))) 20)
      (`self.PickupItem`))))

(event `/Game/DynamicContent/Engine/Inventory/ActionInterface.DropAction`
  (params (`Item To Drop` :type "Actor Object Reference"))
  ;[1 1 1] Inventory Menu
  ;;[1 1 1] Drop Item
  (`self.SetActorHiddenInGame` `Item To Drop` false)
  (`self.SetActorEnableCollision` `Item To Drop` true)
  (`self.K2_SetActorTransform` `Item To Drop` (`KismetMathLibrary.MakeTransform` (+ (.location (`SceneComponent.K2_GetComponentToWorld` (`self.DropLocation`))) (0.0 50.0 100.0)) (.rotation (`SceneComponent.K2_GetComponentToWorld` (`self.DropLocation`))) (.scale (`SceneComponent.K2_GetComponentToWorld` (`self.DropLocation`)))) false false))

(event `Key|T`
  (params (Key :type "Key Structure"))
  (bind _returnvalue (`GameplayStatics.GetPlayerController` 0))
  ;[1 1 1] Crafter Menu
  (:`Pressed`
    (`/Engine/EditorBlueprintResources/StandardMacros.IsValid` (`self.CrafterMenuReference`)
      (:`Is Valid`
        _)
      (:`Is Not Valid`
        (bind _returnvalue_2 (`|CreateWidget` "/Game/DynamicContent/UI/InGame/Crafter.Crafter_C"))
        (bind _output_get (set `self.CrafterMenuReference` _returnvalue_2))))
    (`WidgetBlueprintLibrary.SetInputMode_UIOnlyEx` _returnvalue _output_get)
    (`UserWidget.AddToViewport` _output_get 0)
    (set `PlayerController.bShowMouseCursor` true _returnvalue)))

(event `Key|U`
  (params (Key :type "Key Structure"))
  (bind _returnvalue (`GameplayStatics.GetPlayerController` 0))
  ;[1 1 1] Upgrade Menu
  (:`Pressed`
    (`/Engine/EditorBlueprintResources/StandardMacros.IsValid` (`self.UpgradeMenuReference`)
      (:`Is Valid`
        _)
      (:`Is Not Valid`
        (bind _returnvalue_2 (`|CreateWidget` "/Game/DynamicContent/UI/InGame/Upgrade.Upgrade_C"))
        (bind _output_get (set `self.UpgradeMenuReference` _returnvalue_2))))
    (`WidgetBlueprintLibrary.SetInputMode_UIOnlyEx` _returnvalue _output_get)
    (`UserWidget.AddToViewport` _output_get 0)
    (set `PlayerController.bShowMouseCursor` true _returnvalue)))

(event `Key|N`
  (params (Key :type "Key Structure"))
  (bind _returnvalue (`GameplayStatics.GetPlayerController` 0))
  ;[1 1 1] Map
  (:`Pressed`
    (`/Engine/EditorBlueprintResources/StandardMacros.IsValid` (`self.MapMenuReference`) :!label _label
      (:`Is Valid`
        _)
      (:`Is Not Valid`
        (bind _returnvalue_2 (`|CreateWidget` "/Game/DynamicContent/UI/InGame/Map.Map_C"))
        (bind _output_get (set `self.MapMenuReference` _returnvalue_2))))
    (`WidgetBlueprintLibrary.SetInputMode_UIOnlyEx` _returnvalue _output_get)
    (`UserWidget.AddToViewport` _output_get 0)
    (set `PlayerController.bShowMouseCursor` true _returnvalue)))

(event `ForceOpenMap`
  (goto _label))

(event `Key|Backslash`
  (params (Key :type "Key Structure"))
  ;[1 1 1] Debug
  (:`Pressed`
    (`/Engine/EditorBlueprintResources/StandardMacros.IsValid` (`self.DebugUIReference`)
      (:`Is Valid`
        _)
      (:`Is Not Valid`
        (bind _returnvalue (`|CreateWidget` "/Game/DynamicContent/UI/InGame/Debug.Debug_C"))
        (bind _output_get (set `self.DebugUIReference` _returnvalue))))
    (`/Engine/EditorBlueprintResources/StandardMacros.FlipFlop`
      (:`A`
        (`Widget.RemoveFromParent` _output_get))
      (:`B`
        (`UserWidget.AddToViewport` _output_get 0)))))

(fn `DisableMouseCursor`
  (bind _returnvalue (`GameplayStatics.GetPlayerController` 0))
  (`WidgetBlueprintLibrary.SetInputMode_GameOnly` _returnvalue)
  (bind _asspace_horror_hud (cast `SpaceHorrorHUD` (`PlayerController.GetHUD` _returnvalue)))
  (set `SpaceHorrorHUD.bShowCrosshair` true _asspace_horror_hud)
  (set `PlayerController.bShowMouseCursor` false _returnvalue))

(fn `EnebleMouseCursor`
  (bind _returnvalue (`GameplayStatics.GetPlayerController` 0))
  (`WidgetBlueprintLibrary.SetInputMode_GameAndUIEx` _returnvalue (`self.InventoryMenuReference`))
  (bind _asspace_horror_hud (cast `SpaceHorrorHUD` (`PlayerController.GetHUD` _returnvalue)))
  (set `SpaceHorrorHUD.bShowCrosshair` false _asspace_horror_hud)
  (set `PlayerController.bShowMouseCursor` true _returnvalue))

(fn `ItemChooser`
  (params (ItemID :type Integer))
  (returns (`Item Info` :type "/Game/DynamicContent/Engine/Inventory/InventoryStruct Structure") (IsEmpty :type Boolean))
  (if (== ItemID 1001)
    (return (make `/Game/DynamicContent/Engine/Inventory/InventoryStruct` 1001 null "/Game/StaticContent/StarterContent/Shapes/Shape_Cylinder.Shape_Cylinder" "/Game/DynamicContent/Engine/Inventory/DummyThumbnails/Can.Can" "Painkiller" "Use Painkiller" 20.0) false)
    (elif (== ItemID 1002)
      (return (make `/Game/DynamicContent/Engine/Inventory/InventoryStruct` 1002 null "/Game/StaticContent/StarterContent/Shapes/Shape_Pipe_180.Shape_Pipe_180" "/Game/DynamicContent/Engine/Inventory/DummyThumbnails/Banana.Banana" "Banana" "Eat Banana" 20.0) false)
      (elif (== ItemID 1003)
        (return (make `/Game/DynamicContent/Engine/Inventory/InventoryStruct` 1003 null "/Game/StaticContent/StarterContent/Shapes/Shape_Torus.Shape_Torus" "/Game/DynamicContent/Engine/Inventory/DummyThumbnails/donut.donut" "Donut" "Eat Donut" 10.0) false)
        (elif (== ItemID 1004)
          (return (make `/Game/DynamicContent/Engine/Inventory/InventoryStruct` 1004 null "/Game/StaticContent/StarterContent/Props/MaterialSphere.MaterialSphere" "/Game/DynamicContent/Engine/Inventory/DummyThumbnails/Orange.Orange" "Orange" "Eat Orange" 10.0) false)
          (else
            (return (struct) true)))))))

(fn `ItemConstructer`
  ;[1 1 1] Banana
  (set `self.ItemBanana` (make `/Game/DynamicContent/Engine/Inventory/InventoryStruct` 1001 null null "/Game/DynamicContent/Engine/Inventory/DummyThumbnails/Banana.Banana" "Banana" "Eat Banana"))
  ;[1 1 1] Can
  (set `self.ItemCan` (make `/Game/DynamicContent/Engine/Inventory/InventoryStruct` 1002 null null "/Game/DynamicContent/Engine/Inventory/DummyThumbnails/Can.Can" "Soup Can" "Eat Soup"))
  ;[1 1 1] Donut
  (set `self.ItemDonut` (make `/Game/DynamicContent/Engine/Inventory/InventoryStruct` 1003 null null "/Game/DynamicContent/Engine/Inventory/DummyThumbnails/donut.donut" "Donut" "Eat Donut")))

(fn `SetPlayerDataFromSave`
  (params (SaveReference :type "/Game/DynamicContent/Engine/Save/SaveStruct Structure"))
  (bind (_totalhp _hp _bladder _nap _hunger _curerntbattery _totalbattery _inventory _weapon _craftinventory _currentmission _currentroom _killcount _bosskillcount _deathcount _travelcount _playtime _bladdercount _submissioncount _napcount _eatcount _achievementcount _skillweakspot _skillrunner _skilleater _skillsurvivor _playerprofile) (break `/Game/DynamicContent/Engine/Save/SaveStruct` SaveReference))
  (bind _inventorymenureference (`self.InventoryMenuReference`))
  ;[1 1 1] Set Player Information / Stats / Story / Skill
  (set `self.TotalHP` _totalhp)
  (set `self.HP` _hp)
  (set `self.Bladder` _bladder)
  (set `self.Nap` _nap)
  (set `self.Hunger` _hunger)
  (set `self.TotalBattery` _totalbattery)
  (set `self.CurrentMission` _currentmission)
  (set `self.CurrentRoom` _currentroom)
  (set `self.KillCount` _killcount)
  (set `self.BossKillCount` _bosskillcount)
  (set `self.DeathCount` _deathcount)
  (set `self.TravelCount` _travelcount)
  (set `self.PlayTime` _playtime)
  (set `self.BladderCount` _bladdercount)
  (set `self.SubMissionCount` _submissioncount)
  (set `self.NapCount` _napcount)
  (set `self.EatCount` _eatcount)
  (set `self.Achievement` _achievementcount)
  (set `self.SkillWeakSpot` _skillweakspot)
  (set `self.SkillRunner` _skillrunner)
  (set `self.SkillEater` _skilleater)
  (set `self.SkillSurvivor` _skillsurvivor)
  (set `self.PlayerProfile` _playerprofile)
  ;;[1 1 1] Load Current Ammo each Weapon
  (bind _asbp_wp_door_cutter (cast `/Game/DynamicContent/Weapons/BP_WP_DoorCutter` (`ChildActorComponent.ChildActor` (`self.DC_Gun`))))
  (set `MasterWeapons.uCurrentAmmo` (`|GetArrayItem` _curerntbattery) _asbp_wp_door_cutter)
  (bind _asbp_wp_gauss_rifle (cast `/Game/DynamicContent/Weapons/BP_WP_GaussRifle` (`ChildActorComponent.ChildActor` (`self.GR_Gun`))))
  (set `MasterWeapons.uCurrentAmmo` (`|GetArrayItem` _curerntbattery 1) _asbp_wp_gauss_rifle)
  (bind _asbp_wp_force_gun (cast `/Game/DynamicContent/Weapons/BP_WP_ForceGun` (`ChildActorComponent.ChildActor` (`self.FORCE_Gun`))))
  (set `MasterWeapons.uCurrentAmmo` (`|GetArrayItem` _curerntbattery 2) _asbp_wp_force_gun)
  (bind _asbp_wp_laser (cast `/Game/DynamicContent/Weapons/BP_WP_Laser` (`ChildActorComponent.ChildActor` (`self.LASER_Gun`))))
  (set `MasterWeapons.uCurrentAmmo` (`|GetArrayItem` _curerntbattery 3) _asbp_wp_laser)
  (bind _asbp_wp_rail_gun (cast `/Game/DynamicContent/Weapons/BP_WP_RailGun` (`ChildActorComponent.ChildActor` (`self.RAIL_Gun`))))
  (set `MasterWeapons.uCurrentAmmo` (`|GetArrayItem` _curerntbattery 4) _asbp_wp_rail_gun)
  (bind _asbp_wp_stun_gun (cast `/Game/DynamicContent/Weapons/BP_WP_StunGun` (`ChildActorComponent.ChildActor` (`self.STUN_Gun`))))
  (set `MasterWeapons.uCurrentAmmo` (`|GetArrayItem` _curerntbattery 5) _asbp_wp_stun_gun)
  ;;[1 1 1] Load Item to Inventory
  (for _array_element _inventory
    (bind (_item_info _isempty) (`self.ItemChooser` _array_element))
    (if (not _isempty)
      (bind _structout (`self.SpawnItemActor` _item_info))
      (`KismetArrayLibrary.Array_Add` (`/Game/DynamicContent/UI/InGame/Inventory.Inventory` _inventorymenureference) _structout)
      (`/Game/DynamicContent/UI/InGame/Inventory.RefreshInventory` _inventorymenureference)
      ;;[1 1 1] Load Weapons Variant
      (set `MasterWeapons.weaponVariant` (`|GetArrayItem` _weapon) _asbp_wp_door_cutter)
      (set `MasterWeapons.weaponVariant` (`|GetArrayItem` _weapon 1) _asbp_wp_gauss_rifle)
      (set `MasterWeapons.weaponVariant` (`|GetArrayItem` _weapon 2) _asbp_wp_force_gun)
      (set `MasterWeapons.weaponVariant` (`|GetArrayItem` _weapon 3) _asbp_wp_laser)
      (set `MasterWeapons.weaponVariant` (`|GetArrayItem` _weapon 4) _asbp_wp_rail_gun)
      (set `MasterWeapons.weaponVariant` (`|GetArrayItem` _weapon 5) _asbp_wp_stun_gun)
      ;;[1 1 1] Load Craft Item
      (for (_array_element_2 _array_index) _craftinventory
        (`KismetArrayLibrary.Array_Set` (`self.CraftInventory`) _array_index _array_element_2)))))

(fn `SetupPlayer`
  (bind _returnvalue (`GameplayStatics.GetPlayerController` 0))
  ;[1 1 1] Setup HP
  (set `self.HP` (`self.TotalHP`))
  (`self.UpdateHealth` false)
  ;[1 1 1] Create HUD
  (bind _returnvalue_2 (`|CreateWidget` "/Game/DynamicContent/UI/InGame/HUD.HUD_C" _returnvalue)) ; set hud to playerone (not reccommend for multiplayer)
  (bind _output_get (set `self.HudReference` _returnvalue_2))
  (`UserWidget.AddToViewport` _output_get 0)
  (`WidgetBlueprintLibrary.SetInputMode_GameOnly` _returnvalue)
  ;[1 1 1] Pre Create Inventory for Load Inventory Stuff
  (bind _returnvalue_3 (`|CreateWidget` "/Game/DynamicContent/UI/InGame/Inventory.Inventory_C"))
  (set `self.InventoryMenuReference` _returnvalue_3)
  ;[1 1 1] Call after Complete Setup
  (`self.OnSetupReferenceComplete`)
  ;[1 1 1] Add Debug Widget
  (bind _returnvalue_4 (`|CreateWidget` "/Game/DynamicContent/UI/InGame/Debug.Debug_C"))
  (bind _output_get_2 (set `self.DebugUIReference` _returnvalue_4))
  (`UserWidget.AddToViewport` _output_get_2 0))

(fn `SpawnItemActor`
  (params (ItemStruct :type "/Game/DynamicContent/Engine/Inventory/InventoryStruct Structure"))
  (returns (StructOut :type "/Game/DynamicContent/Engine/Inventory/InventoryStruct Structure (by ref)"))
  (bind (_itemid _item _itemmesh _itemimage _pickuptext _actiontext _addhealth) (break `/Game/DynamicContent/Engine/Inventory/InventoryStruct` ItemStruct))
  (bind _asbp_master_items (castclass `/Game/DynamicContent/Engine/Inventory/BP_MasterItems` "/Game/DynamicContent/Engine/Inventory/BP_MasterItems.BP_MasterItems_C"))
  (bind _returnvalue (`|SpawnActorFromClass` _asbp_master_items (`KismetMathLibrary.MakeTransform` (-3000.0 -1000.0 30.0)) "AlwaysSpawn" "OverrideRootScale" null null))
  (`self.SetActorEnableCollision` _returnvalue true)
  (`SceneComponent.SetHiddenInGame` (`Actor.RootComponent` _returnvalue) false false)
  (bind _output_get (set `/Game/DynamicContent/Engine/Inventory/BP_MasterItems.ItemInfo` (make `/Game/DynamicContent/Engine/Inventory/InventoryStruct` _itemid _returnvalue _itemmesh _itemimage _pickuptext _actiontext _addhealth) _returnvalue))
  (message `/Game/DynamicContent/Engine/Inventory/ActionInterface.LoadItemInformation` _returnvalue)
  (return _output_get))

(fn `TakeDamage`
  (set `self.HP` (- (`self.HP`) 20.0))
  (`self.UpdateHealth` false))

(fn `UpdateHealth`
  (params (logHealth :type Boolean) (logPercent :type Boolean))
  (returns (HealthPercent :type "Float (double-precision)"))
  (bind _hp (`self.HP`))
  (bind _output_get (set `self.HeathPercent` (/ _hp (`self.TotalHP`))))
  (`KismetSystemLibrary.PrintString` (`KismetStringLibrary.Conv_DoubleToString` _hp) logHealth logHealth)
  (`KismetSystemLibrary.PrintString` (`KismetStringLibrary.Conv_DoubleToString` _output_get) logPercent logPercent)
  (return _output_get))

(fn `UserConstructionScript`
  (`self.ItemConstructer`))